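; Shared orthographic camera actor that keeps the players passed to SetCurrentPlayers framed on the side-view XZ plane.
; Each Tick it gathers player X and Z positions, sets ortho width, then centers the camera between the extremes using Y and Z offsets.
; Width is the largest of MinWidth and the buffered X and 16:9-scaled Z spreads, each spread taken modulo MaxWidth rather than clamped.
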(event Custom|Set%20Current%20Players
  (params (in%20Characters :type Array%20of%20Character%20BP%20Object%20References))
  (Variables|Default|SetPlayers in%20Characters))

(event EventBeginPlay)

(event Collision|EventActorBeginOverlap
  (params (OtherActor :type Actor%20Object%20Reference)))

(event EventTick
  (params (DeltaSeconds :type Float%20%28single-precision%29))
  (CallFunction|UpdateCamera))

(fn ConstructionScript
  (bind _game_camera (Variables|Default|GetGame%20Camera))
  (bind _defaultsceneroot (Variables|Default|GetDefaultSceneRoot))
  (bind _returnvalue (Transformation|GetWorldLocation _defaultsceneroot))
  (bind _returnvalue_2 (Transformation|GetWorldLocation _game_camera))
  (bind (_x _y _z) (Math|Vector|BreakVector _returnvalue))
  (bind (_x_2 _y_2 _z_2) (Math|Vector|BreakVector _returnvalue_2))
  (Transformation|SetWorldLocation (Variables|Default|GetDefaultSceneRoot) (Math|Vector|MakeVector _x 0.0 _z) false false)
  (Transformation|SetWorldLocation (Variables|Default|GetGame%20Camera) (Math|Vector|MakeVector _x_2 (Variables|Default|GetCamera%20Y%20Offset) _z_2) false false))

(fn UpdateCamera
  (|StorePlayerLocations)
  (|SetOrthoWidth)
  (|SetCameraPosition))