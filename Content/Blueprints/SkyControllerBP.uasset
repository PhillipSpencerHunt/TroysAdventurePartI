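; SkyControllerBP is a sky actor that blends the sky's look and continuously rotates its stars.
; The construction script creates a dynamic instance of DayMaterial on SkyMesh.
; UpdateSkyController sets that material's Alpha parameter and moves the root to a supplied world location.
; Tick stores delta time, which RotateStars uses to turn StarsPivot at a frame-rate-independent degrees-per-second speed.
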(event Custom|Update%20Sky%20Controller
  (params (Sky%20Alpha :type Float%20%28single-precision%29) (New%20World%20Location :type Vector))
  (Rendering|Material|SetScalarParameterValue (Variables|Default|GetSky%20Material) "Alpha" Sky%20Alpha :!class /Script/Engine.MaterialInstanceDynamic)
  (Transformation|SetWorldLocation (Variables|Default|GetDefaultSceneRoot) New%20World%20Location false false))

(event EventBeginPlay)

(event Collision|EventActorBeginOverlap
  (params (OtherActor :type Actor%20Object%20Reference)))

(event EventTick
  (params (DeltaSeconds :type Float%20%28single-precision%29))
  (Variables|Default|SetTime%20Tick DeltaSeconds)
  (Utilities|RotateStars))

(fn ConstructionScript
  (bind _returnvalue (Rendering|Material|CreateDynamicMaterialInstance (Variables|Default|GetSkyMesh) 0 "/Game/Materials/DayMaterial.DayMaterial" :!class /Script/Engine.PrimitiveComponent))
  (Variables|Default|SetSky%20Material _returnvalue))