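; Menu controller actor that runs the main menu for local multiplayer, handling player joins, menu input, level launch and quit.
; On BeginPlay it creates the menu widget and loads available characters from a GameData save.
; A MenuState enum routes Start presses into character selection or creation and gates forwarded up, down and activate input by joined or acting player.
; Settings and credits events only print, and temp-player spawning is disconnected.
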(event Custom|Menu%20Press%20Activate
  (params (Player :type Character%20BP%20Object%20Reference))
  (Variables|Default|SetInput%20Player 0)
  (Utilities|HasPlayerJoined? (Variables|Default|GetInput%20Player)
    (:Yes
      (Utilities|CanPlayerPress? (Variables|Default|GetInput%20Player)
        (:Yes
          (Default|Activate (Variables|Default|GetMain%20Menu%20Widget%20Instance)))))))

(event Custom|Menu%20Press%20Up
  (params (Player :type Character%20BP%20Object%20Reference))
  (Variables|Default|SetInput%20Player Player)
  (Utilities|HasPlayerJoined? (Variables|Default|GetInput%20Player)
    (:Yes
      (Utilities|CanPlayerPress? (Variables|Default|GetInput%20Player)
        (:Yes
          (Default|UpArrow (Variables|Default|GetMain%20Menu%20Widget%20Instance)))))))

(event Custom|Menu%20Press%20Down
  (params (Player :type Character%20BP%20Object%20Reference))
  (Variables|Default|SetInput%20Player 0)
  (Utilities|HasPlayerJoined? (Variables|Default|GetInput%20Player)
    (:Yes
      (Utilities|CanPlayerPress? (Variables|Default|GetInput%20Player)
        (:Yes
          (Default|DownArrow (Variables|Default|GetMain%20Menu%20Widget%20Instance)))))))

(event Custom|Play%20Game
  (Development|PrintString "Play" false)
  (CallFunction|RemovePlayersandPawns)
  (Game|OpenLevel(byName) "TestingMap"))

(event Custom|Player%20Press%20Start
  (params (Player :type Character%20BP%20Object%20Reference))
  ;[1 1 1] A player Presses the "Start" Button
  (CallFunction|PressStart Player))

(event Custom|Open%20Credits
  (Development|PrintString "Open Credits" false))

(event Custom|Open%20Settings
  (params (Player :type Character%20BP%20Object%20Reference))
  (Development|PrintString "Open Settings" false))

(event Custom|Exit%20game
  (params (Player :type Character%20BP%20Object%20Reference))
  (Development|PrintString "Quit Game" false)
  (Game|QuitGame 0 "Quit"))

(event EventBeginPlay
  (CallFunction|AddMenu)
  (CallFunction|LoadGameData)
  (switch Utilities|FlowControl|Switch|SwitchonMenuState (Variables|MenuOptions|GetMenu%20State)))

(event Collision|EventActorBeginOverlap
  (params (OtherActor :type Actor%20Object%20Reference)))

(event EventTick
  (params (DeltaSeconds :type Float%20%28single-precision%29)))

(fn ConstructionScript)

(fn AddTempPlayers
  ;[1 1 1] Create remaining 3 players
  (for _index (range 1 3)
    (Class|GameplayStatics|CreatePlayer _index))
  ;[1 1 1] Add the players
  (for _index_2 (range 0 3)
    (bind _ascharacter_bp (Utilities|Casting|CastToCharacterBP (Game|Player|GetPlayerPawn _index_2)))
    (Default|SetControllerNumber _ascharacter_bp _index_2)
    (Transformation|SetWorldLocation (Variables|/Script/Engine.Character|GetCapsuleComponent _ascharacter_bp) (Utilities|Array|Get(acopy) (Variables|PlayerLocations|GetPlayer%20Start%20Locations) _index_2) false false)
    (Utilities|Array|Add (Variables|Default|GetTemp%20Players) _ascharacter_bp)))

(fn AddMenu
  (bind _returnvalue (Game|ConstructObjectfromClass "/Game/Widgets/MenuWidget.MenuWidget_C" (Game|GetPlayerController 0)))
  (Variables|Default|SetMain%20Menu%20Widget%20Instance _returnvalue)
  (Default|SetMainMenuControllerInstance (Variables|Default|GetMain%20Menu%20Widget%20Instance) self)
  (UserInterface|Viewport|AddtoViewport (Variables|Default|GetMain%20Menu%20Widget%20Instance) 0)
  (switch Utilities|FlowControl|Switch|SwitchonMenuState (Variables|MenuOptions|GetMenu%20State)
    (:NewEnumerator1
      (Default|ShowMainMenu (Variables|Default|GetMain%20Menu%20Widget%20Instance)))
    (:NewEnumerator6
      (Widget|SetVisibility (Variables|Default|GetMain%20Menu%20Widget%20Instance) "Hidden"))))

(fn RemovePlayersandPawns
  (for _array_element (Variables|Default|GetTemp%20Players)
    (Class|GameplayStatics|RemovePlayer (Game|GetPlayerController (Variables|/Game/Blueprints/CharacterBP.CharacterBP_C|GetPlayer%20Controller%20Number _array_element)) true)))

(fn LoadGameData
  (bind _returnvalue (SaveGame|CreateSaveGameObject "/Game/Data/GameData.GameData_C"))
  (bind _output_get (Variables|Default|SetGame%20Data%20Instance _returnvalue))
  (bind _returnvalue_2 (SaveGame|LoadGamefromSlot (Variables|/Game/Data/GameData.GameData_C|GetSave%20Slot%20Name _output_get) (Variables|/Game/Data/GameData.GameData_C|GetUser%20Index _output_get)))
  (bind _asgame_data (Utilities|Casting|CastToGameData _returnvalue_2))
  (bind _output_get_2 (Variables|Default|SetGame%20Data%20Instance _asgame_data))
  (Variables|Default|SetAvailable%20Characters (Variables|/Game/Data/GameData.GameData_C|GetAll%20Characters _output_get_2))
  (Development|PrintString (Utilities|String|Append (Utilities|String|ToString(Integer) (Utilities|Array|Length (Variables|/Game/Data/GameData.GameData_C|GetAll%20Characters _output_get_2))) " characters loaded.") false))

(fn SaveCharacters)

(fn InitializeCharacters
  (bind _returnvalue (SaveGame|CreateSaveGameObject "/Game/Data/GameData.GameData_C"))
  (bind _output_get (Variables|Default|SetGame%20Data%20Instance _returnvalue))
  (Variables|/Game/Data/GameData.GameData_C|SetSave%20Date _output_get (Math|DateTime|Now))
  (bind _returnvalue_2 (SaveGame|SaveGametoSlot _output_get (Variables|/Game/Data/GameData.GameData_C|GetSave%20Slot%20Name _output_get) (Variables|/Game/Data/GameData.GameData_C|GetUser%20Index _output_get)))
  (if _returnvalue_2
    (Development|PrintString "Saved Successfully." false)
    (else
      (Development|PrintString "Failed to Save." false))))

(fn LoadPlayingCharacters
  (for _array_element (Variables|/Game/Data/GameData.GameData_C|GetPlaying%20Characters (Variables|Default|GetGame%20Data%20Instance))
    _))

(fn OpenSelectCharacter
  (Variables|MenuOptions|SetMenu%20State "NewEnumerator2")
  (Default|ShowCharacterSelection (Variables|Default|GetMain%20Menu%20Widget%20Instance)))

(fn OpenCreateCharacter
  (Variables|MenuOptions|SetMenu%20State "NewEnumerator3")
  (Default|ShowCharacterMaker (Variables|Default|GetMain%20Menu%20Widget%20Instance)))

(fn PressStart
  (params (Player :type Character%20BP%20Object%20Reference))
  (LocalVariables|SetTrying%20Player Player)
  (switch Utilities|FlowControl|Switch|SwitchonMenuState (Variables|MenuOptions|GetMenu%20State)
    (:NewEnumerator1
      (Utilities|HasPlayerJoined? (Variables|Default|GetActing%20Player)
        (:No
          (if (< (Utilities|Array|Length (Variables|Default|GetJoined%20Players)) (Variables|Default|GetMax%20Players))
            (bind _returnvalue (Utilities|Array|Add (Variables|Default|GetJoined%20Players) (Variables|Default|GetActing%20Player)))
            (Default|ConnectPlayer (Variables|Default|GetMain%20Menu%20Widget%20Instance) (+ _returnvalue 1))
            (if (> (Utilities|Array|Length (Variables|Default|GetAvailable%20Characters)) 0)
              (CallFunction|OpenSelectCharacter)
              (else
                (CallFunction|OpenCreateCharacter)))
            (Variables|Default|SetActing%20Player (LocalVariables|GetTrying%20Player))
            (return)))))
    (:NewEnumerator2
      (Development|PrintString (Utilities|String|Append "Do nothing with start in " (Utilities|String|EnumtoString (Variables|MenuOptions|GetMenu%20State))) false :!label _label))
    (:NewEnumerator3
      (goto _label))
    (:NewEnumerator4
      (goto _label))
    (:NewEnumerator8
      (goto _label))))