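; Game controller actor that runs the day/night cycle and, on the main menu, sets up temporary local players.
; Each tick advances a minute/second clock and samples day-to-night or night-to-day curves for sky alpha.
; It passes that alpha to the SkyController, with a position tracking camera X/Z at fixed Y depth.
; Menu setup creates extra players, places four characters at start locations and registers them with the shared GameCameraController.
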(event EventBeginPlay
  (Utilities|Array|Clear (Variables|PlayerSettings|GetActual%20Players))
  (if (Variables|Coordinatorsettings|GetIs%20Main%20Menu)
    (Utilities|UseTempPlayers)))

(event Collision|EventActorBeginOverlap
  (params (OtherActor :type Actor%20Object%20Reference)))

(event EventTick
  (params (DeltaSeconds :type Float%20%28single-precision%29))
  (Utilities|UpdateGameTime DeltaSeconds
    (:out
      (Camera|GetCameraLocation)
      (|UpdateSkyLocation)
      (Default|UpdateSkyController (Variables|CoordinatorSettings|GetSky%20Controller) (Variables|GameTime|GetCurrent%20Sky%20Alpha) (Variables|Default|GetSky%20Location)))))

(fn ConstructionScript
  (Variables|GameTime|SetLength%20of%20a%20Day%20%28min%29 (+ (Variables|GameTime|GetLength%20of%20Daylight%20%28min%29) (Variables|GameTime|GetLength%20of%20Night%20%28min%29))))